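; BP_NPC_NavMesh is a wandering NPC that shows a jumpscare when the player touches it.
; From BeginPlay, MoveNPC loops: AI Move To a random reachable navmesh point nearby, beep and pause on arrival, or retry almost immediately on failure.
; Capsule overlap with BP_FirstPersonCharacter adds a new Jumpscare widget to the viewport and prints a debug message, independently of the movement loop.
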(event `self.ReceiveBeginPlay`
  (`self.MoveNPC`))

(event `MoveNPC`
  (bind _output_get (set `self.Random Location` (`NavigationSystemV1.K2_GetRandomReachablePointInRadius` (`self.K2_GetActorLocation`) 1000.0 null null)))
  (`|AIMoveTo` self _output_get null
    (:`OnSuccess`
      (`GameplayStatics.PlaySoundAtLocation` "/Game/audio/beep-sound-8333.beep-sound-8333" (`SceneComponent.K2_GetComponentLocation` (`self.CapsuleComponent`)) (struct) 1.0 1.0 0.0 null null null null)
      (`KismetSystemLibrary.Delay` 2.0)
      (`self.MoveNPC`))
    (:`OnFail`
      (`KismetSystemLibrary.Delay` 0.1)
      (`self.MoveNPC`))))

(event `self.CapsuleComponent.OnComponentBeginOverlap`
  (params (OverlappedComponent :type "PrimitiveComponent Object Reference") (OtherActor :type "Actor Object Reference") (OtherComp :type "PrimitiveComponent Object Reference") (OtherBodyIndex :type Integer) (bFromSweep :type Boolean) (SweepResult :type "HitResult Structure (by ref)"))
  (cast `/Game/FirstPerson/Blueprints/BP_FirstPersonCharacter` OtherActor)
  (bind _returnvalue (`|CreateWidget` "/Game/widgets/jumpscare.jumpscare_C"))
  (`UserWidget.AddToViewport` _returnvalue 0)
  (`KismetSystemLibrary.PrintText` "Hello"))

(fn `UserConstructionScript`)